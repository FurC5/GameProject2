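; Riddle piece item for the final puzzle that can be grabbed, dropped, attached and inspected.
; When BP_FinalPuzzle interacts, the piece detaches for inspection if the puzzle holds an object, otherwise it attaches to the puzzle's attachment point.
; Pressing Inspection ends inspection and reattaches it to the puzzle.
; Grab notifies any previous owner through IBP_Interactions, disabling collision only for FirstPersonCharacter owners; Drop restores collision.
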(event `self.Drop`
  (`self.Detach`)
  (`PrimitiveComponent.SetCollisionEnabled` (`self.StaticMesh`) "QueryAndPhysics"))

(event `self.Grab`
  (params (Owner :type "Actor Object Reference") (AttachmentPoint :type "SceneComponent Object Reference"))
  (bind _output_get (set `self.AttachmentComponent` AttachmentPoint))
  (if (`KismetSystemLibrary.DoesImplementInterface` (`self.AttachementOwner`) "/Game/Blueprint/Puzzles/IBP_Interactions.IBP_Interactions_C")
    (message `/Game/Blueprint/Puzzles/IBP_Interactions.Detach` (`self.AttachementOwner`))
    (`self.Detach`))
  (`self.Attach` _output_get Owner)
  (cast `/Game/Blueprint/Player/FirstPersonCharacter` Owner)
  (`PrimitiveComponent.SetCollisionEnabled` (`self.StaticMesh`) "NoCollision"))

(event `self.PawnInteractWith`
  (params (Pawn :type "Pawn Object Reference"))
  (bind _output_get (set `self.OwnerPawn` Pawn))
  (bind _asbp_final_puzzle (cast `/Game/Blueprint/Puzzles/FinalPuzzle/BP_FinalPuzzle` _output_get))
  (`/Game/Blueprint/Puzzles/FinalPuzzle/BP_FinalPuzzle.AttachedObject` _asbp_final_puzzle
    (:`then`
      (`self.K2_DetachFromActor` "KeepWorld" "KeepWorld" "KeepWorld")
      (`self.Inspect` 20.0))
    (:`else`
      (`self.Grab` _asbp_final_puzzle (`/Game/Blueprint/Puzzles/FinalPuzzle/BP_FinalPuzzle.AttachmentPoint` _asbp_final_puzzle))
      (`self.Stop inspect` (0.0 0.0 0.0) (`SceneComponent.K2_GetComponentRotation` (`self.StaticMesh`))))))

(event `self.Attach`
  (params (Component :type "SceneComponent Object Reference") (Actor :type "Actor Object Reference"))
  (`self.K2_AttachToComponent` Component "None" "SnapToTarget" "KeepWorld" "KeepWorld")
  (`PrimitiveComponent.SetSimulatePhysics` (`self.StaticMesh`) false)
  (set `self.AttachementOwner` Actor))

(event `InputAction|Inspection`
  (params (Key :type "Key Structure"))
  (:`Pressed`
    (bind _asbp_final_puzzle (cast `/Game/Blueprint/Puzzles/FinalPuzzle/BP_FinalPuzzle` (`self.OwnerPawn`)))
    (`self.Attach` (`/Game/Blueprint/Puzzles/FinalPuzzle/BP_FinalPuzzle.AttachmentPoint` _asbp_final_puzzle) _asbp_final_puzzle)
    (`self.Stop inspect` (0.0 0.0 0.0) (`SceneComponent.K2_GetComponentRotation` (`self.StaticMesh`)))))

(event `self.Detach`
  (`self.K2_DetachFromActor` "KeepWorld" "KeepWorld" "KeepWorld")
  (set `self.AttachementOwner` null)
  (`KismetSystemLibrary.PrintString` "Detach Successful"))

(fn `UserConstructionScript`
  (`parent.UserConstructionScript`))