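; Manager actor that keeps a capped number of randomly chosen paintings swapped in the environment.
; On begin play it registers itself with every available painting.
; Each tick below the cap, it picks from the available pool, parking already-rendered paintings in a rendered list and messaging others to swap.
; Paintings report back when swapped to normal or no longer rendered, returning them to the available pool.
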(event `self.ReceiveBeginPlay`
  (for _array_element (`self.AvailPaint`)
    (set `/Game/Blueprint/Environment/BP_SwappingPaintings.Managr` self _array_element)))

(event `self.ReceiveTick`
  (params (DeltaSeconds :type "Float (single-precision)"))
  (bind _availpaint (`self.AvailPaint`))
  (bind _output (`|GetArrayItem` _availpaint (`KismetMathLibrary.RandomInteger` (`KismetArrayLibrary.Array_Length` _availpaint))))
  (if (== (`KismetArrayLibrary.Array_Length` (`self.SwapPaint`)) (`self.MaxNumSwap`))
    _
    (elif (> (`KismetArrayLibrary.Array_Length` (`self.AvailPaint`)) 0)
      (if (`/Game/Blueprint/Environment/BP_SwappingPaintings.HasBeenRendered` _output)
        (`KismetArrayLibrary.Array_Add` (`self.RenderPaint`) _output)
        (`KismetArrayLibrary.Array_RemoveItem` _availpaint _output)
        (else
          (message `/Game/Blueprint/Environment/IBP_Swap.SwapPainting` _output)
          (`KismetArrayLibrary.Array_Add` (`self.SwapPaint`) _output)
          (`KismetArrayLibrary.Array_RemoveItem` (`self.AvailPaint`) _output)))
      (else
        (`KismetSystemLibrary.PrintString` "Hello" true true (struct :`G` 0.66 :`B` 1.0 :`A` 1.0) 0.1)))))

(event `/Game/Blueprint/Environment/IBP_Swap.HasSwappedToNormal`
  (params (Painting :type "/Game/Blueprint/Environment/BP_SwappingPaintings Object Reference"))
  (`self.SwapPaintingBetweenArray` Painting (`self.SwapPaint`) (`self.AvailPaint`)))

(event `/Game/Blueprint/Environment/IBP_Swap.IsNotRendered`
  (params (Painting :type "/Game/Blueprint/Environment/BP_SwappingPaintings Object Reference"))
  (`self.SwapPaintingBetweenArray` Painting (`self.RenderPaint`) (`self.AvailPaint`)))

(fn `UserConstructionScript`)