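; BP_AudioPlayer is an environment actor that plays a configurable sound when activated.
; BeginPlay assigns SoundToPlay to its Audio component.
; Activate starts playback only if the sound is not already playing, and Deactivate stops it.
; AddInt and Attach are stubs that return false, with no key, puzzle or attachment logic.
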(event `self.ReceiveBeginPlay`
  (`AudioComponent.SetSound` (`self.Audio`) (`self.SoundToPlay`)))

(event `/Game/Blueprint/Puzzles/IBP_Interactions.Activate`
  (if (not (`AudioComponent.IsPlaying` (`self.Audio`)))
    (`AudioComponent.Play` (`self.Audio`) 0.0)))

(event `/Game/Blueprint/Puzzles/IBP_Interactions.Deactivate`
  (`AudioComponent.Stop` (`self.Audio`)))

(fn `AddInt`
  (params (KeyCode :type Integer))
  (returns (CorrectKey :type Boolean) (PuzzleCompleted :type Boolean))
  (return false false))

(fn `Attach`
  (params (Actor :type "/Game/Blueprint/BP_ItemParent Object Reference") (Inspection :type "/Game/Blueprint/Inspecting/BP_InspectionObject_1 Object Reference"))
  (returns (Attached :type Boolean))
  (return false))

(fn `UserConstructionScript`)