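; BP_SwappingPaintings is an environment painting that swaps between normal and scary materials on its Cube while out of view.
; A looping timer rolls a percentage chance to apply the scary material, only while the painting is not flagged as rendered.
; Tick uses WasRecentlyRendered to track visibility, restoring the normal material once a seen painting leaves view.
; Debug strings print the render state every tick and each scary swap.
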(event `self.ReceiveTick`
  (params (DeltaSeconds :type "Float (single-precision)"))
  (if (`self.WasRecentlyRendered` 0.1)
    (`KismetSystemLibrary.PrintString` "I'm rendered!")
    (set `self.HasBeenRendered` true)
    (else
      (`KismetSystemLibrary.PrintString` "Where did I go?")
      (if (`self.HasBeenRendered`)
        (set `self.HasBeenRendered` false)
        (if (`self.IsScary`)
          (`PrimitiveComponent.SetMaterial` (`self.Cube`) 0 (`self.NormalMaterial`))
          (set `self.IsScary` false))))))

(event `self.ReceiveBeginPlay`
  (`KismetSystemLibrary.K2_SetTimerDelegate` (delegate `TestToSwap`) (`self.TimeToSwapable`) true))

(event `TestToSwap`
  (if (and (<= (`KismetMathLibrary.RandomFloat`) (/ (`self.ChanceToSwap`) 100.0)) (not (`self.IsScary`)) (== (`self.HasBeenRendered`) false))
    (`KismetSystemLibrary.PrintString` "Make Scary")
    (`PrimitiveComponent.SetMaterial` (`self.Cube`) 0 (`self.ScaryMaterial`))
    (set `self.IsScary` true)))

(fn `UserConstructionScript`)