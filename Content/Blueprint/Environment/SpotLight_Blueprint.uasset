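; Spotlight Blueprint that starts hidden and flickers once an actor overlaps its trigger box.
; The first overlap starts a looping timer that calls ToggleLights, which flips the light's visibility and randomizes its intensity between Probability and NewVar0.
; NewVar0 also sets the timer interval.
; End overlap hides the light but never clears the timer, so toggling continues.
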(event `self.ReceiveBeginPlay`
  (`SceneComponent.SetVisibility` (`self.SpotLightComponent`) false false)
  (set `self.Lighting` false))

(event `self.TriggerLightBox.OnActorBeginOverlap`
  (params (OverlappedActor :type "Actor Object Reference") (OtherActor :type "Actor Object Reference"))
  (if (not (`KismetSystemLibrary.K2_TimerExistsHandle` (`self.LightToggleHandle`)))
    (bind _returnvalue (`KismetSystemLibrary.K2_SetTimer` self "ToggleLights" (`self.NewVar_0`) true))
    (set `self.LightToggleHandle` _returnvalue)))

(event `self.TriggerLightBox.OnActorEndOverlap`
  (params (OverlappedActor :type "Actor Object Reference") (OtherActor :type "Actor Object Reference"))
  (`SceneComponent.SetVisibility` (`self.SpotLightComponent`) false false))

(fn `ToggleLights`
  (`SceneComponent.SetVisibility` (`self.SpotLightComponent`) (not (`SceneComponent.IsVisible` (`self.SpotLightComponent`))) false)
  (`LightComponent.SetIntensity` (`self.SpotLightComponent`) (`KismetMathLibrary.RandomFloatInRange` (`self.probability`) (`self.NewVar_0`))))

(fn `UserConstructionScript`)