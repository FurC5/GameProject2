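; BP_TheRunningMan is an activatable ghost runner that moves a static mesh along a spline at constant speed with audible footsteps.
; Tick advances the mesh while active, then at the spline's end messages actor lists to activate or deactivate and stops itself.
; A looping timer traces below the mesh, alternating left and right ghost footstep sounds at the hit point, with random creaks on wood floors.
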(event `/Game/Blueprint/Puzzles/IBP_Interactions.Activate`
  (set `self.Active` true))

(event `self.ReceiveTick`
  (params (DeltaSeconds :type "Float (single-precision)"))
  (set `self.Delta` DeltaSeconds)
  (if (`self.Active`)
    (`|ExecutionSequence`
      (:`then_0`
        (if (>= (`self.CurrentDistanceDownSpline`) (`SplineComponent.GetSplineLength` (`self.Spline`)))
          (for _array_element (`self.ActorsToActivate`)
            (message `/Game/Blueprint/Puzzles/IBP_Interactions.Activate` _array_element))
          (for _array_element_2 (`self.ActorsToDeactivate`)
            (message `/Game/Blueprint/Puzzles/IBP_Interactions.Deactivate` _array_element_2))
          (set `self.Active` false)))
      (:`then_1`
        (`self.MoveObject`))
      (:`then_2`
        (`/Engine/EditorBlueprintResources/StandardMacros.DoOnce` false :!label _label
          (:`Completed`
            (bind _returnvalue (`KismetSystemLibrary.K2_SetTimer` self "DoMovementSounds" (`self.TimeBetweenStepSound`) true))
            (set `self.SoundTimer` _returnvalue)))))
    (else
      (`|ExecutionSequence`
        (:`then_0`
          (goto _label :!via `Reset`))
        (:`then_1`
          (`KismetSystemLibrary.K2_ClearAndInvalidateTimerHandle` (`self.SoundTimer`)))))))

(event `MoveObject`
  (bind _returnvalue_location (`KismetMathLibrary.BreakTransform` (`SplineComponent.GetTransformAtDistanceAlongSpline` (`self.Spline`) (`self.CurrentDistanceDownSpline`) "World" false)))
  (set `self.CurrentDistanceDownSpline` (+ (`self.CurrentDistanceDownSpline`) (* (`self.MovementSpeed`) (`self.Delta`))))
  (`SceneComponent.K2_SetWorldLocation` (`self.StaticMesh`) _returnvalue_location false false))

(fn `AddInt`
  (params (KeyCode :type Integer))
  (returns (CorrectKey :type Boolean) (PuzzleCompleted :type Boolean))
  (return false false))

(fn `Attach`
  (params (Actor :type "/Game/Blueprint/BP_ItemParent Object Reference") (Inspection :type "/Game/Blueprint/Inspecting/BP_InspectionObject_1 Object Reference"))
  (returns (Attached :type Boolean))
  (return false))

(fn `DoMovementSounds`
  (bind _returnvalue (`SceneComponent.K2_GetComponentLocation` (`self.StaticMesh`)))
  (bind (_outhit _returnvalue_2) (`KismetSystemLibrary.LineTraceSingle` _returnvalue (- _returnvalue (0.0 0.0 150.0)) "TraceTypeQuery1"))
  (if _returnvalue_2
    (`|ExecutionSequence`
      (:`then_0`
        (`/Engine/EditorBlueprintResources/StandardMacros.FlipFlop`
          (:`A`
            (bind (_bblockinghit _binitialoverlap _time _distance _location) (`GameplayStatics.BreakHitResult` _outhit))
            (`GameplayStatics.PlaySoundAtLocation` "/Game/Audio/SoundFX/Environment/Indoor/Footstep/GhostFootstep/Variant_1/S_V1_LEFT_GhostFootsteps_Cue.S_V1_LEFT_GhostFootsteps_Cue" _location (struct) 1.0 1.0 0.0 null null null))
          (:`B`
            (`GameplayStatics.PlaySoundAtLocation` "/Game/Audio/SoundFX/Environment/Indoor/Footstep/GhostFootstep/Variant_1/S_V1_RIGHT_GhostFootstep_Cue.S_V1_RIGHT_GhostFootstep_Cue" _location (struct) 1.0 1.0 0.0 null null null))))
      (:`then_1`
        (switch `EPhysicalSurface` (`GameplayStatics.GetSurfaceType` _outhit)
          (:`SurfaceType1`
            (if (<= (`KismetMathLibrary.RandomInteger` 100) (`self.ChanceForWoodCreak`))
              (`GameplayStatics.PlaySoundAtLocation` "/Game/Audio/SoundFX/Environment/Indoor/Wood/S_WoodSteps_Cue.S_WoodSteps_Cue" _location (struct) 1.0 1.0 0.0 "/Game/Audio/SoundFX/Environment/Outdoors/Rain/AT_RainArea.AT_RainArea" null null))))))))

(fn `UserConstructionScript`)