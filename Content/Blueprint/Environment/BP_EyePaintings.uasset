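; BP_EyePaintings is an unfinished painting actor with left and right eye components, marked in its graph as not working.
; The construction script stores each eye's world location as a start position.
; BeginPlay waits briefly, then caches the controlled FirstPersonCharacter as Player or prints an error.
; Tick runs an empty sequence, and a disconnected node would set the right eye's relative location, so the eyes never move.
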(event `self.ReceiveBeginPlay`
  ;[1 1 1] None of this works
  (`KismetSystemLibrary.Delay` 0.2)
  (bind _asfirst_person_character (cast `/Game/Blueprint/Player/FirstPersonCharacter` (`Controller.K2_GetPawn` (`GameplayStatics.GetPlayerController` 0)))
    (:`then`
      (set `self.Player` _asfirst_person_character))
    (:`CastFailed`
      (`KismetSystemLibrary.PrintString` "Controller Actor NOT a FirstPersonCharacter" true true (struct :`R` 1.0 :`A` 1.0)))))

(event `self.ReceiveTick`
  (params (DeltaSeconds :type "Float (single-precision)"))
  ;[1 1 1] None of this works
  (`|ExecutionSequence`))

(fn `UserConstructionScript`
  (set `self.R_Eye_StartPos` (`SceneComponent.K2_GetComponentLocation` (`self.R_PaintingEye`)))
  (set `self.L_Eye_StartPos` (`SceneComponent.K2_GetComponentLocation` (`self.L_PaintingEye`))))