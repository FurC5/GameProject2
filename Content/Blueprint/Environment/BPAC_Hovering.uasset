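; BPAC_Hovering is an actor component that, judging by its name, is meant to make items hover, though it applies no movement yet.
; BeginPlay stores the owner's starting location as Origin, which nothing here reads.
; Each Tick line-traces straight down from the owner by TraceLength on the Visibility channel.
; On a hit it casts the owner to BP_ItemParent, and the logic ends there.
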(event `self.ReceiveTick`
  (params (DeltaSeconds :type "Float (single-precision)"))
  (bind _returnvalue (`Actor.K2_GetActorLocation` (`self.GetOwner`)))
  (bind (_outhit _returnvalue_2) (`KismetSystemLibrary.LineTraceSingle` _returnvalue (- _returnvalue (`KismetMathLibrary.MakeVector` 0.0 0.0 (`self.TraceLength`))) "TraceTypeQuery1"))
  (if _returnvalue_2
    (cast `/Game/Blueprint/BP_ItemParent` (`self.GetOwner`))))

(event `self.ReceiveBeginPlay`
  (set `self.Origin` (`Actor.K2_GetActorLocation` (`self.GetOwner`))))