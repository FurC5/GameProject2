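; Game-over sequence pawn that, when activated, takes over player control and plays a scripted ending before loading a level.
; After a delay, a timeline eases its root rotation toward zero and raises it to 50 units above its starting position.
; It then sends an activate message to the linked doors, fades the camera out and opens L_LayoutBlockOut_kat.
; AddInt and Attach are stubs that return false.
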(event `self.ReceiveBeginPlay`
  (set `self.TargetPos` (+ (`SceneComponent.K2_GetComponentLocation` (`self.DefaultSceneRoot`)) (0.0 0.0 50.0))))

(event `/Game/Blueprint/Puzzles/IBP_Interactions.Activate`
  (bind _defaultsceneroot (`self.DefaultSceneRoot`))
  (`Controller.Possess` (`GameplayStatics.GetPlayerController` 0) self)
  (`KismetSystemLibrary.Delay` (`self.LookUpDelay`))
  (bind (_direction _alpha) (`Timeline|LookUpTimeline`)
    (:`Update`
      (`SceneComponent.K2_SetWorldRotation` _defaultsceneroot (`KismetMathLibrary.RLerp` (`SceneComponent.K2_GetComponentRotation` _defaultsceneroot) (struct) _alpha true) false false)
      (`SceneComponent.K2_SetWorldLocation` _defaultsceneroot (`KismetMathLibrary.VLerp` (`SceneComponent.K2_GetComponentLocation` (`self.DefaultSceneRoot`)) (`self.TargetPos`) _alpha) false false))
    (:`Finished`
      (`KismetSystemLibrary.Delay` (`self.DoorOpenDelay`))
      (for _array_element (`self.DoorsToOpen`)
        (message `/Game/Blueprint/Puzzles/IBP_Interactions.Activate` _array_element))
      (`PlayerCameraManager.StartCameraFade` :`self` (`GameplayStatics.GetPlayerCameraManager` 0) :`ToAlpha` 1.0 :`Duration` (`self.TimeToFade`) :`bHoldWhenFinished` true)
      (`KismetSystemLibrary.Delay` (+ (`self.TimeToFade`) 3.0))
      (`GameplayStatics.OpenLevel` "L_LayoutBlockOut_kat"))))

(fn `AddInt`
  (params (KeyCode :type Integer))
  (returns (CorrectKey :type Boolean) (PuzzleCompleted :type Boolean))
  (return false false))

(fn `Attach`
  (params (Actor :type "/Game/Blueprint/BP_ItemParent Object Reference") (Inspection :type "/Game/Blueprint/Inspecting/BP_InspectionObject_1 Object Reference"))
  (returns (Attached :type Boolean))
  (return false))

(fn `UserConstructionScript`)