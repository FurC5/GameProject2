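; Lightning light Blueprint that flashes a light component to a given intensity and fades it back down.
; UpdateLights sets the intensity directly, while ResetLights only raises a Resetting flag.
; Tick subtracts a fixed amount every frame regardless of delta time or the flag, snapping to zero and clearing the flag only when Resetting is set and intensity is near zero.
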(event `/Game/Blueprint/Environment/IBP_Lightning.UpdateLights`
  (params (NewIntensity :type "Float (single-precision)"))
  (`LightComponent.SetIntensity` (`self.LightComponent`) NewIntensity))

(event `/Game/Blueprint/Environment/IBP_Lightning.ResetLights`
  (set `self.Resetting` true))

(event `self.ReceiveTick`
  (params (DeltaSeconds :type "Float (single-precision)"))
  (bind _lightcomponent (`self.LightComponent`))
  (if (and (`KismetMathLibrary.NearlyEqual_FloatFloat` (`LightComponentBase.Intensity` _lightcomponent) 0.0 0.1) (`self.Resetting`))
    (`LightComponent.SetIntensity` _lightcomponent 0.0)
    (set `self.Resetting` false)
    (else
      (`LightComponent.SetIntensity` _lightcomponent (- (`LightComponentBase.Intensity` _lightcomponent) 1000.0)))))

(fn `UserConstructionScript`)