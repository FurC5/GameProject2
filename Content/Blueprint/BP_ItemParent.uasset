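; BP_ItemParent is a base item actor that can be grabbed, attached to an owner's component, and dropped.
; Grab stores the attachment point and, if the current holder implements IBP_Interactions, sends it DetachMessage and detaches before attaching to the new owner.
; Attach snaps the item to the component and disables mesh physics.
; Detach, also called by Drop, keeps world transform, re-enables physics and clears the owner.
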(event `/Game/Blueprint/IBP_Grabable.Drop`
  (`self.Detach`))

(event `/Game/Blueprint/IBP_Grabable.Grab`
  (params (Owner :type "Actor Object Reference") (AttachmentPoint :type "SceneComponent Object Reference"))
  (bind _output_get (set `self.AttachmentComponent` AttachmentPoint))
  (if (`KismetSystemLibrary.DoesImplementInterface` (`self.AttachementOwner`) "/Game/Blueprint/Puzzles/IBP_Interactions.IBP_Interactions_C")
    (message `/Game/Blueprint/Puzzles/IBP_Interactions.Detach` (`self.AttachementOwner`))
    (`self.Detach`))
  (`self.Attach` _output_get Owner))

(event `Detach`
  (`self.K2_DetachFromActor` "KeepWorld" "KeepWorld" "KeepWorld")
  (`PrimitiveComponent.SetSimulatePhysics` (`self.StaticMesh`) true)
  (set `self.AttachementOwner` null)
  (`KismetSystemLibrary.PrintString` "Detach Successful"))

(event `Attach`
  (params (Component :type "SceneComponent Object Reference") (Actor :type "Actor Object Reference"))
  (`self.K2_AttachToComponent` Component "None" "SnapToTarget" "SnapToTarget" "KeepWorld")
  (`PrimitiveComponent.SetSimulatePhysics` (`self.StaticMesh`) false)
  (set `self.AttachementOwner` Actor))

(fn `UserConstructionScript`)