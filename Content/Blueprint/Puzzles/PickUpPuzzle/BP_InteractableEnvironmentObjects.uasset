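; Interactable environment object for the pick-up puzzle that reveals linked items and triggers other actors when interacted with.
; It hides the linked Key and disables its physics and collision at BeginPlay.
; When Interactable, EnvironmentalInteract reveals the assigned note and Key with collision and sound, and sends ActivateMessage to linked actors, each once.
; DeactivateMessage goes to its listed actors on every interaction, with no DoOnce guard.
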(event `self.ReceiveBeginPlay`
  (bind _key (`self.Key`))
  (bind _staticmesh (`/Game/Blueprint/BP_ItemParent.StaticMesh` _key))
  (if (!= (`self.Key`) null)
    (`SceneComponent.SetVisibility` (`Actor.RootComponent` _key) false false)
    (`PrimitiveComponent.SetSimulatePhysics` _staticmesh false)
    (`PrimitiveComponent.SetCollisionEnabled` _staticmesh "NoCollision")))

(event `/Game/Blueprint/IBP_Grabable.EnvironmentalInteract`
  (params (Player :type "/Game/Blueprint/Player/FirstPersonCharacter Object Reference"))
  (bind _notetospawn (`self.NoteToSpawn`))
  (bind _key (`self.Key`))
  (bind _staticmesh (`/Game/Blueprint/BP_ItemParent.StaticMesh` _notetospawn))
  (if (`self.Interactable`)
    (if (!= (`self.NoteToSpawn`) null)
      (`/Engine/EditorBlueprintResources/StandardMacros.DoOnce` false
        (:`Completed`
          (`SceneComponent.SetVisibility` (`Actor.RootComponent` _notetospawn) true false)
          (`PrimitiveComponent.SetSimulatePhysics` _staticmesh false)
          (`PrimitiveComponent.SetCollisionEnabled` _staticmesh "QueryAndPhysics")
          (`GameplayStatics.PlaySoundAtLocation` (`self.ActivationSound`) (`self.K2_GetActorLocation` (`self.NoteToSpawn`)) (struct) 1.0 1.0 0.0 null null null))))
    (if (!= (`self.Key`) null)
      (`/Engine/EditorBlueprintResources/StandardMacros.DoOnce` false
        (:`Completed`
          (`SceneComponent.SetVisibility` (`Actor.RootComponent` _key) true false)
          (`PrimitiveComponent.SetCollisionEnabled` (`/Game/Blueprint/BP_ItemParent.StaticMesh` _key) "QueryAndPhysics")
          (`GameplayStatics.PlaySoundAtLocation` (`self.ActivationSound`) (`self.K2_GetActorLocation` (`self.Key`)) (struct) 1.0 1.0 0.0 null null null))))
    (if (> (`KismetArrayLibrary.Array_Length` (`self.ActorsToActivate`)) 0)
      (`/Engine/EditorBlueprintResources/StandardMacros.DoOnce` false
        (:`Completed`
          (for _array_element (`self.ActorsToActivate`)
            (message `/Game/Blueprint/Puzzles/IBP_Interactions.Activate` _array_element)))))
    (if (> (`KismetArrayLibrary.Array_Length` (`self.ActorsToDeactivate`)) 0)
      (for _array_element_2 (`self.ActorsToDeactivate`)
        (message `/Game/Blueprint/Puzzles/IBP_Interactions.Deactivate` _array_element_2)))))

(fn `UserConstructionScript`)