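; Pickup puzzle piece item that, when interacted with, unlocks another object and reveals an optional key.
; On BeginPlay it can hide itself through HideObject, and it hides any assigned Key, switching off that key's physics and collision.
; Interacting runs the parent's interaction, marks ObjectToInteractWith as interactable, and shows the Key with physics-only collision while leaving its physics simulation off.
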(event `self.ReceiveBeginPlay`
  (bind _staticmesh (`self.StaticMesh`))
  (bind _key (`self.Key`))
  (bind _staticmesh_2 (`/Game/Blueprint/BP_ItemParent.StaticMesh` _key))
  (if (`self.HideObject?`)
    (`SceneComponent.SetVisibility` _staticmesh false false)
    (`PrimitiveComponent.SetSimulatePhysics` _staticmesh false)
    (`PrimitiveComponent.SetCollisionEnabled` _staticmesh "NoCollision"))
  (if (!= (`self.Key`) null)
    (`SceneComponent.SetVisibility` (`Actor.RootComponent` _key) false false)
    (`PrimitiveComponent.SetSimulatePhysics` _staticmesh_2 false)
    (`PrimitiveComponent.SetCollisionEnabled` _staticmesh_2 "NoCollision")))

(event `/Game/Blueprint/IBP_Grabable.InteractWith`
  (params (PlayerCharacter :type "/Game/Blueprint/Player/FirstPersonCharacter Object Reference"))
  (bind _key (`self.Key`))
  (bind _staticmesh (`/Game/Blueprint/BP_ItemParent.StaticMesh` _key))
  (`parent.InteractWith` PlayerCharacter)
  (if (!= (`self.ObjectToInteractWith`) null)
    (set `/Game/Blueprint/Puzzles/PickUpPuzzle/BP_InteractableEnvironmentObjects.Interactable` true (`self.ObjectToInteractWith`)))
  (if (!= (`self.Key`) null)
    (`SceneComponent.SetVisibility` (`Actor.RootComponent` _key) true false)
    (`PrimitiveComponent.SetSimulatePhysics` _staticmesh false)
    (`PrimitiveComponent.SetCollisionEnabled` _staticmesh "PhysicsOnly")))

(fn `UserConstructionScript`
  (`parent.UserConstructionScript`))