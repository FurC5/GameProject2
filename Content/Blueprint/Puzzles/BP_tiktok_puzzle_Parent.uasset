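; Parent puzzle pawn that the player possesses through Enter and leaves with U, returning control to the stored character.
; While left mouse is held, Tick accumulates an angle from an input axis and rotates the Sphere around its local Y axis via axis-angle.
; StopGimbalLock only recenters the shown cursor each dragging tick, despite its name, and the world rotation is printed for debugging.
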(event `Key|U`
  (params (Key :type "Key Structure"))
  ;[1 1 1] Posses 'n unPosses
  (:`Pressed`
    (`Controller.Possess` (`GameplayStatics.GetPlayerController` 0) (`self.PlayerCharacter`))))

(event `/Game/Blueprint/Puzzles/PianoPuzzle/BPI_Enter.Enter`
  (params (Player :type "/Game/Blueprint/Player/FirstPersonCharacter Object Reference"))
  ;[1 1 1] Posses 'n unPosses
  (set `self.PlayerCharacter` Player)
  (`Controller.Possess` (`GameplayStatics.GetPlayerController` 0) self))

(event `Key|LeftMouseButton`
  (params (Key :type "Key Structure"))
  ;[1 1 1] Rotate
  (:`Pressed`
    (set `self.isDraging` true))
  (:`Released`
    (set `self.isDraging` false)))

(event `self.ReceiveTick`
  (params (DeltaSeconds :type "Float (single-precision)"))
  ;[1 1 1] Rotate
  (if (`self.isDraging`)
    (set `PlayerController.bShowMouseCursor` true (`GameplayStatics.GetPlayerController` 0))
    (set `self.currentAngle` (+ (`self.currentAngle`) (* 2 (`self.GetInputAxisKeyValue`))))
    (`SceneComponent.K2_SetRelativeRotation` (`self.Sphere`) (`KismetMathLibrary.RotatorFromAxisAndAngle` (0.0 1.0 0.0) (`self.currentAngle`)) false false)
    (`self.StopGimbalLock`)
    (`KismetSystemLibrary.PrintString` (`KismetStringLibrary.Conv_RotatorToString` (`SceneComponent.K2_GetComponentRotation` (`self.Sphere`))))))

(fn `StopGimbalLock`
  (bind (_returnvalue_x _returnvalue_y) (`KismetMathLibrary.BreakVector2D` (`WidgetLayoutLibrary.GetViewportSize`)))
  (`PlayerController.SetMouseLocation` (`GameplayStatics.GetPlayerController` 0) (`KismetMathLibrary.FTrunc` (/ _returnvalue_x 2.0)) (`KismetMathLibrary.FTrunc` (/ _returnvalue_y 2.0)))
  (return))

(fn `UserConstructionScript`)