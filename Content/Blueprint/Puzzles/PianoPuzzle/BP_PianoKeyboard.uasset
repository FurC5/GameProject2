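; Playable piano keyboard pawn for the piano puzzle: Enter possesses it, and M hands control back to the player character.
; The construction script maps key components to start position, key code and down state, which keyboard input toggles.
; Every Tick, PlayKey interpolates each key's position, uses DoOnce gates to play its note once per press, fades it on release, and passes key codes to PuzzleOwner through AddIntMessage.
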(event `/Game/Blueprint/Puzzles/PianoPuzzle/BPI_Enter.Enter`
  (params (Player :type "/Game/Blueprint/Player/FirstPersonCharacter Object Reference"))
  ;[1 1 1] Possession of Piano
  (set `self.PlayerCharacter` Player)
  (`Controller.Possess` (`GameplayStatics.GetPlayerController` 0) self))

(event `Key|M`
  (params (Key :type "Key Structure"))
  ;[1 1 1] Possession of Piano
  (:`Pressed`
    (`Controller.Possess` (`GameplayStatics.GetPlayerController` 0) (`self.PlayerCharacter`))))

(event `Key|A`
  (params (Key :type "Key Structure"))
  ;[1 1 1] Key Registration Purgatory
  (:`Pressed`
    (`self.UpdateIsDown` (`self.Key:F`) :!label _label))
  (:`Released`
    (goto _label :!via `False`)))

(event `Key|S`
  (params (Key :type "Key Structure"))
  ;[1 1 1] Key Registration Purgatory
  (:`Pressed`
    (`self.UpdateIsDown` (`self.Key:G`) :!label _label_2))
  (:`Released`
    (goto _label_2 :!via `False`)))

(event `Key|D`
  (params (Key :type "Key Structure"))
  ;[1 1 1] Key Registration Purgatory
  (:`Pressed`
    (`self.UpdateIsDown` (`self.Key:A`) :!label _label_3))
  (:`Released`
    (goto _label_3 :!via `False`)))

(event `Key|F`
  (params (Key :type "Key Structure"))
  ;[1 1 1] Key Registration Purgatory
  (:`Pressed`
    (`self.UpdateIsDown` (`self.Key:B`) :!label _label_4))
  (:`Released`
    (goto _label_4 :!via `False`)))

(event `Key|G`
  (params (Key :type "Key Structure"))
  ;[1 1 1] Key Registration Purgatory
  (:`Pressed`
    (`self.UpdateIsDown` (`self.Key:C`) :!label _label_5))
  (:`Released`
    (goto _label_5 :!via `False`)))

(event `Key|H`
  (params (Key :type "Key Structure"))
  ;[1 1 1] Key Registration Purgatory
  (:`Pressed`
    (`self.UpdateIsDown` (`self.Key:D`) :!label _label_6))
  (:`Released`
    (goto _label_6 :!via `False`)))

(event `Key|J`
  (params (Key :type "Key Structure"))
  ;[1 1 1] Key Registration Purgatory
  (:`Pressed`
    (`self.UpdateIsDown` (`self.Key:E`) :!label _label_7))
  (:`Released`
    (goto _label_7 :!via `False`)))

(event `Key|K`
  (params (Key :type "Key Structure"))
  ;[1 1 1] Key Registration Purgatory
  (:`Pressed`
    (`self.UpdateIsDown` (`self.Key:F2`) :!label _label_8))
  (:`Released`
    (goto _label_8 :!via `False`)))

(event `Key|L`
  (params (Key :type "Key Structure"))
  ;[1 1 1] Key Registration Purgatory
  (:`Pressed`
    (`self.UpdateIsDown` (`self.Key:G2`) :!label _label_9))
  (:`Released`
    (goto _label_9 :!via `False`)))

(event `self.ReceiveTick`
  (params (DeltaSeconds :type "Float (single-precision)"))
  ;[1 1 1] Key Playing hell
  (set `self.DeltaTime` DeltaSeconds)
  (`|ExecutionSequence`
    (:`then_0`
      (bind _keycode (`self.PlayKey` (`self.Key:F`) (`self.DeltaTime`) (`self.Key:F_AudioComponent`)))
      (message `/Game/Blueprint/Puzzles/IBP_Interactions.AddInt` (`self.PuzzleOwner`) _keycode))
    (:`then_1`
      (bind _keycode_2 (`self.PlayKey` (`self.Key:G`) (`self.DeltaTime`) (`self.Key:G_AudioComponent`)))
      (message `/Game/Blueprint/Puzzles/IBP_Interactions.AddInt` (`self.PuzzleOwner`) _keycode_2))
    (:`then_2`
      (bind _keycode_3 (`self.PlayKey` (`self.Key:A`) (`self.DeltaTime`) (`self.Key:A_AudioComponent`)))
      (message `/Game/Blueprint/Puzzles/IBP_Interactions.AddInt` (`self.PuzzleOwner`) _keycode_3))
    (:`then_3`
      (bind _keycode_4 (`self.PlayKey` (`self.Key:B`) (`self.DeltaTime`) (`self.Key:B_AudioComponent`)))
      (message `/Game/Blueprint/Puzzles/IBP_Interactions.AddInt` (`self.PuzzleOwner`) _keycode_4))
    (:`then_4`
      (bind _keycode_5 (`self.PlayKey` (`self.Key:C`) (`self.DeltaTime`) (`self.Key:C_AudioComponent`)))
      (message `/Game/Blueprint/Puzzles/IBP_Interactions.AddInt` (`self.PuzzleOwner`) _keycode_5))
    (:`then_5`
      (bind _keycode_6 (`self.PlayKey` (`self.Key:D`) (`self.DeltaTime`) (`self.Key:D_AudioComponent`)))
      (message `/Game/Blueprint/Puzzles/IBP_Interactions.AddInt` (`self.PuzzleOwner`) _keycode_6))
    (:`then_6`
      (bind _keycode_7 (`self.PlayKey` (`self.Key:E`) (`self.DeltaTime`) (`self.Key:E_AudioComponent`)))
      (message `/Game/Blueprint/Puzzles/IBP_Interactions.AddInt` (`self.PuzzleOwner`) _keycode_7))
    (:`then_7`
      (bind _keycode_8 (`self.PlayKey` (`self.Key:F2`) (`self.DeltaTime`) (`self.Key:F2_AudioComponent`)))
      (message `/Game/Blueprint/Puzzles/IBP_Interactions.AddInt` (`self.PuzzleOwner`) _keycode_8))
    (:`then_8`
      (bind _keycode_9 (`self.PlayKey` (`self.Key:G2`) (`self.DeltaTime`) (`self.Key:G2_AudioComponent`)))
      (message `/Game/Blueprint/Puzzles/IBP_Interactions.AddInt` (`self.PuzzleOwner`) _keycode_9))
    (:`then_9`
      (bind _keycode_10 (`self.PlayKey` (`self.Key:A2`) (`self.DeltaTime`) (`self.Key:A2_AudioComponent`)))
      (message `/Game/Blueprint/Puzzles/IBP_Interactions.AddInt` (`self.PuzzleOwner`) _keycode_10))
    (:`then_10`
      (bind _keycode_11 (`self.PlayKey` (`self.Key:B2`) (`self.DeltaTime`) (`self.Key:B2_AudioComponent`)))
      (message `/Game/Blueprint/Puzzles/IBP_Interactions.AddInt` (`self.PuzzleOwner`) _keycode_11))
    (:`then_11`
      (bind _keycode_12 (`self.PlayKey` (`self.Key:F#`) (`self.DeltaTime`) (`self.Key:F#_AudioComponent`)))
      (message `/Game/Blueprint/Puzzles/IBP_Interactions.AddInt` (`self.PuzzleOwner`) _keycode_12))
    (:`then_12`
      (bind _keycode_13 (`self.PlayKey` (`self.Key:G#`) (`self.DeltaTime`) (`self.Key:G#_AudioComponent`)))
      (message `/Game/Blueprint/Puzzles/IBP_Interactions.AddInt` (`self.PuzzleOwner`) _keycode_13))
    (:`then_13`
      (bind _keycode_14 (`self.PlayKey` (`self.Key:A#`) (`self.DeltaTime`) (`self.Key:A#_AudioComponent`)))
      (message `/Game/Blueprint/Puzzles/IBP_Interactions.AddInt` (`self.PuzzleOwner`) _keycode_14))
    (:`then_14`
      (bind _keycode_15 (`self.PlayKey` (`self.Key:C#`) (`self.DeltaTime`) (`self.Key:C#_AudioComponent`)))
      (message `/Game/Blueprint/Puzzles/IBP_Interactions.AddInt` (`self.PuzzleOwner`) _keycode_15))
    (:`then_15`
      (bind _keycode_16 (`self.PlayKey` (`self.Key:D#`) (`self.DeltaTime`) (`self.Key:D#_AudioComponent`)))
      (message `/Game/Blueprint/Puzzles/IBP_Interactions.AddInt` (`self.PuzzleOwner`) _keycode_16))
    (:`then_16`
      (bind _keycode_17 (`self.PlayKey` (`self.Key:F1#`) (`self.DeltaTime`) (`self.Key:F1#_AudioComponent`)))
      (message `/Game/Blueprint/Puzzles/IBP_Interactions.AddInt` (`self.PuzzleOwner`) _keycode_17))
    (:`then_17`
      (bind _keycode_18 (`self.PlayKey` (`self.Key:G1#`) (`self.DeltaTime`) (`self.Key:G1#_AudioComponent`)))
      (message `/Game/Blueprint/Puzzles/IBP_Interactions.AddInt` (`self.PuzzleOwner`) _keycode_18))
    (:`then_18`
      (bind _keycode_19 (`self.PlayKey` (`self.Key:A1#`) (`self.DeltaTime`) (`self.Key:A1#_AudioComponent`)))
      (message `/Game/Blueprint/Puzzles/IBP_Interactions.AddInt` (`self.PuzzleOwner`) _keycode_19))))

(event `Key|ö`
  (params (Key :type "Key Structure"))
  ;[1 1 1] Key Registration Purgatory
  (:`Pressed`
    (`self.UpdateIsDown` (`self.Key:A2`) :!label _label_10))
  (:`Released`
    (goto _label_10 :!via `False`)))

(event `Key|ä`
  (params (Key :type "Key Structure"))
  ;[1 1 1] Key Registration Purgatory
  (:`Pressed`
    (`self.UpdateIsDown` (`self.Key:B2`) :!label _label_11))
  (:`Released`
    (goto _label_11 :!via `False`)))

(event `Key|W`
  (params (Key :type "Key Structure"))
  ;[1 1 1] Key Registration Purgatory
  (:`Pressed`
    (`self.UpdateIsDown` (`self.Key:F#`) :!label _label_12))
  (:`Released`
    (goto _label_12 :!via `False`)))

(event `Key|E`
  (params (Key :type "Key Structure"))
  ;[1 1 1] Key Registration Purgatory
  (:`Pressed`
    (`self.UpdateIsDown` (`self.Key:G#`) :!label _label_13))
  (:`Released`
    (goto _label_13 :!via `False`)))

(event `Key|R`
  (params (Key :type "Key Structure"))
  ;[1 1 1] Key Registration Purgatory
  (:`Pressed`
    (`self.UpdateIsDown` (`self.Key:A#`) :!label _label_14))
  (:`Released`
    (goto _label_14 :!via `False`)))

(event `Key|T`
  (params (Key :type "Key Structure"))
  ;[1 1 1] Key Registration Purgatory
  (:`Pressed`
    (`self.UpdateIsDown` (`self.Key:C#`) :!label _label_15))
  (:`Released`
    (goto _label_15 :!via `False`)))

(event `Key|Y`
  (params (Key :type "Key Structure"))
  ;[1 1 1] Key Registration Purgatory
  (:`Pressed`
    (`self.UpdateIsDown` (`self.Key:D#`) :!label _label_16))
  (:`Released`
    (goto _label_16 :!via `False`)))

(event `Key|U`
  (params (Key :type "Key Structure"))
  ;[1 1 1] Key Registration Purgatory
  (:`Pressed`
    (`self.UpdateIsDown` (`self.Key:F1#`) :!label _label_17))
  (:`Released`
    (goto _label_17 :!via `False`)))

(event `Key|I`
  (params (Key :type "Key Structure"))
  ;[1 1 1] Key Registration Purgatory
  (:`Pressed`
    (`self.UpdateIsDown` (`self.Key:G1#`) :!label _label_18))
  (:`Released`
    (goto _label_18 :!via `False`)))

(event `Key|O`
  (params (Key :type "Key Structure"))
  ;[1 1 1] Key Registration Purgatory
  (:`Pressed`
    (`self.UpdateIsDown` (`self.Key:A1#`) :!label _label_19))
  (:`Released`
    (goto _label_19 :!via `False`)))

(fn `UserConstructionScript`
  (bind (_outkey _struct_pianokeyinfo) (`self.SetKey` (`self.Key:F`) 0 "/Game/Audio/SoundFX/PianoKeys/SoundCues/S_Piano_F3_Cue.S_Piano_F3_Cue" (`self.Key:F_AudioComponent`)))
  (bind (_outkey_2 _struct_pianokeyinfo_2) (`self.SetKey` (`self.Key:G`) 1 "/Game/Audio/SoundFX/PianoKeys/SoundCues/S_Piano_G3_Cue.S_Piano_G3_Cue" (`self.Key:G_AudioComponent`)))
  (bind (_outkey_3 _struct_pianokeyinfo_3) (`self.SetKey` (`self.Key:A`) 2 "/Game/Audio/SoundFX/PianoKeys/SoundCues/S_Piano_A3_Cue.S_Piano_A3_Cue" (`self.Key:A_AudioComponent`)))
  (bind (_outkey_4 _struct_pianokeyinfo_4) (`self.SetKey` (`self.Key:B`) 3 "/Game/Audio/SoundFX/PianoKeys/SoundCues/S_Piano_B3_Cue.S_Piano_B3_Cue" (`self.Key:B_AudioComponent`)))
  (bind (_outkey_5 _struct_pianokeyinfo_5) (`self.SetKey` (`self.Key:C`) 4 "/Game/Audio/SoundFX/PianoKeys/SoundCues/S_Piano_C4_Cue.S_Piano_C4_Cue" (`self.Key:C_AudioComponent`)))
  (bind (_outkey_6 _struct_pianokeyinfo_6) (`self.SetKey` (`self.Key:D`) 5 "/Game/Audio/SoundFX/PianoKeys/SoundCues/S_Piano_D4_Cue.S_Piano_D4_Cue" (`self.Key:D_AudioComponent`)))
  (bind (_outkey_7 _struct_pianokeyinfo_7) (`self.SetKey` (`self.Key:E`) 6 "/Game/Audio/SoundFX/PianoKeys/SoundCues/S_Piano_E4_Cue.S_Piano_E4_Cue" (`self.Key:E_AudioComponent`)))
  (bind (_outkey_8 _struct_pianokeyinfo_8) (`self.SetKey` (`self.Key:F2`) 7 "/Game/Audio/SoundFX/PianoKeys/SoundCues/S_Piano_F4_Cue.S_Piano_F4_Cue" (`self.Key:F2_AudioComponent`)))
  (bind (_outkey_9 _struct_pianokeyinfo_9) (`self.SetKey` (`self.Key:G#`) 12 "/Game/Audio/SoundFX/PianoKeys/SoundCues/S_Piano_G_3_Cue.S_Piano_G_3_Cue" (`self.Key:G#_AudioComponent`)))
  (bind (_outkey_10 _struct_pianokeyinfo_10) (`self.SetKey` (`self.Key:A#`) 13 "/Game/Audio/SoundFX/PianoKeys/SoundCues/S_Piano_A_3_Cue.S_Piano_A_3_Cue" (`self.Key:A#_AudioComponent`)))
  (bind (_outkey_11 _struct_pianokeyinfo_11) (`self.SetKey` (`self.Key:G2`) 8 "/Game/Audio/SoundFX/PianoKeys/SoundCues/S_Piano_G4_Cue.S_Piano_G4_Cue" (`self.Key:G2_AudioComponent`)))
  (bind (_outkey_12 _struct_pianokeyinfo_12) (`self.SetKey` (`self.Key:C#`) 14 "/Game/Audio/SoundFX/PianoKeys/SoundCues/S_Piano_C_4_Cue.S_Piano_C_4_Cue" (`self.Key:C#_AudioComponent`)))
  (bind (_outkey_13 _struct_pianokeyinfo_13) (`self.SetKey` (`self.Key:D#`) 15 "/Game/Audio/SoundFX/PianoKeys/SoundCues/S_Piano_D_4_Cue.S_Piano_D_4_Cue" (`self.Key:D#_AudioComponent`)))
  (bind (_outkey_14 _struct_pianokeyinfo_14) (`self.SetKey` (`self.Key:A2`) 9 "/Game/Audio/SoundFX/PianoKeys/SoundCues/S_Piano_A4_Cue.S_Piano_A4_Cue" (`self.Key:A2_AudioComponent`)))
  (bind (_outkey_15 _struct_pianokeyinfo_15) (`self.SetKey` (`self.Key:B2`) 10 "/Game/Audio/SoundFX/PianoKeys/SoundCues/S_Piano_B4_Cue.S_Piano_B4_Cue" (`self.Key:B2_AudioComponent`)))
  (bind (_outkey_16 _struct_pianokeyinfo_16) (`self.SetKey` (`self.Key:F#`) 11 "/Game/Audio/SoundFX/PianoKeys/SoundCues/S_Piano_F_3_Cue.S_Piano_F_3_Cue" (`self.Key:F#_AudioComponent`)))
  (bind (_outkey_17 _struct_pianokeyinfo_17) (`self.SetKey` (`self.Key:F1#`) 16 "/Game/Audio/SoundFX/PianoKeys/SoundCues/S_Piano_F_4_Cue.S_Piano_F_4_Cue" (`self.Key:F1#_AudioComponent`)))
  (bind (_outkey_18 _struct_pianokeyinfo_18) (`self.SetKey` (`self.Key:G1#`) 17 "/Game/Audio/SoundFX/PianoKeys/SoundCues/S_Piano_G_4_Cue.S_Piano_G_4_Cue" (`self.Key:G1#_AudioComponent`)))
  (bind (_outkey_19 _struct_pianokeyinfo_19) (`self.SetKey` (`self.Key:A1#`) 18 "/Game/Audio/SoundFX/PianoKeys/SoundCues/S_Piano_A_4_Cue.S_Piano_A_4_Cue" (`self.Key:A1#_AudioComponent`)))
  (bind _output_get (set `self.KeyboardInfo` (`|MakeMap` _outkey _struct_pianokeyinfo _outkey_2 _struct_pianokeyinfo_2 _outkey_3 _struct_pianokeyinfo_3 _outkey_4 _struct_pianokeyinfo_4 _outkey_5 _struct_pianokeyinfo_5 _outkey_6 _struct_pianokeyinfo_6 _outkey_7 _struct_pianokeyinfo_7 _outkey_8 _struct_pianokeyinfo_8 _outkey_11 _struct_pianokeyinfo_11 _outkey_14 _struct_pianokeyinfo_14 _outkey_15 _struct_pianokeyinfo_15 _outkey_16 _struct_pianokeyinfo_16 _outkey_9 _struct_pianokeyinfo_9 _outkey_10 _struct_pianokeyinfo_10 _outkey_12 _struct_pianokeyinfo_12 _outkey_13 _struct_pianokeyinfo_13 _outkey_17 _struct_pianokeyinfo_17 _outkey_18 _struct_pianokeyinfo_18 _outkey_19 _struct_pianokeyinfo_19)))
  (`BlueprintMapLibrary.Map_Keys` _output_get))