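; BP_PianoPuzzle is a sequence puzzle that activates a target object when piano keys are entered in the correct order.
; On BeginPlay it registers itself as the Piano's puzzle owner, and its AddInt event checks each incoming code against PuzzleCode at the current index.
; A match advances the index or, on the last entry, calls ActivateMessage on ObjectToActivate.
; A wrong code resets the sequence, with debug prints reporting progress and resets.
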(event `self.ReceiveBeginPlay`
  (set `/Game/Blueprint/Puzzles/PianoPuzzle/BP_PianoKeyboard.PuzzleOwner` self (`self.Piano`)))

(event `/Game/Blueprint/Puzzles/IBP_Interactions.AddInt`
  (params (Code :type Integer))
  (bind _puzzlecode (`self.PuzzleCode`))
  (bind _puzzleindex (`self.PuzzleIndex`))
  (bind _puzzleindex_2 (`self.PuzzleIndex`))
  (if (or (!= Code (`|GetArrayItem` _puzzlecode _puzzleindex_2)) (< (`KismetArrayLibrary.Array_Length` _puzzlecode) _puzzleindex_2))
    (set `self.PuzzleIndex` 0)
    (`KismetSystemLibrary.PrintString` "Wrong key, reset sequence...")
    (elif (== (`KismetArrayLibrary.Array_LastIndex` (`self.PuzzleCode`)) _puzzleindex)
      (message `/Game/Blueprint/Puzzles/IBP_Interactions.Activate` (`self.ObjectToActivate`))
      (else
        (`KismetSystemLibrary.PrintString` (`KismetTextLibrary.Conv_TextToString` (`|FormatText` "Right key more needed. \nThis was: {I}" _puzzleindex)))
        (`/Engine/EditorBlueprintResources/StandardMacros.IncrementInt` _puzzleindex)))))

(fn `UserConstructionScript`)