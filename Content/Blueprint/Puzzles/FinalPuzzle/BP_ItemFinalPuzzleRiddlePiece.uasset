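; A riddle piece for the final puzzle that can be grabbed, dropped, inspected and attached to BP_FinalPuzzle.
; On interaction from the puzzle, it detaches and opens inspection if an object is already attached, otherwise it snaps to the puzzle's attachment point.
; Grabbing notifies any previous owner through IBP_Interactions and disables collision for FirstPersonCharacter, while dropping restores it.
; The Inspection input attaches the piece to the puzzle and ends inspection.
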(event `self.Drop`
  (`self.FinalRiddleDetach`)
  (`PrimitiveComponent.SetCollisionEnabled` (`self.StaticMesh`) "QueryAndPhysics"))

(event `self.Grab`
  (params (Owner :type "Actor Object Reference") (AttachmentPoint :type "SceneComponent Object Reference"))
  (bind _output_get (set `self.AttachmentComponent` AttachmentPoint))
  (if (`KismetSystemLibrary.DoesImplementInterface` (`self.AttachementOwner`) "/Game/Blueprint/Puzzles/IBP_Interactions.IBP_Interactions_C")
    (message `/Game/Blueprint/Puzzles/IBP_Interactions.Detach` (`self.AttachementOwner`))
    (`self.FinalRiddleDetach`))
  (`self.FinalRiddleAttach` _output_get Owner)
  (cast `/Game/Blueprint/Player/FirstPersonCharacter` Owner)
  (`PrimitiveComponent.SetCollisionEnabled` (`self.StaticMesh`) "NoCollision"))

(event `self.PawnInteractWith`
  (params (Pawn :type "Pawn Object Reference"))
  (bind _output_get (set `self.OwnerPawn` Pawn))
  (bind _asbp_final_puzzle (cast `/Game/Blueprint/Puzzles/FinalPuzzle/BP_FinalPuzzle` _output_get))
  (`/Game/Blueprint/Puzzles/FinalPuzzle/BP_FinalPuzzle.AttachedObject` _asbp_final_puzzle
    (:`then`
      (`self.K2_DetachFromActor` "KeepWorld" "KeepWorld" "KeepWorld")
      (`self.Inspect` 20.0))
    (:`else`
      (`self.Grab` _asbp_final_puzzle (`/Game/Blueprint/Puzzles/FinalPuzzle/BP_FinalPuzzle.AttachmentPoint` _asbp_final_puzzle))
      (`self.Stop inspect` (0.0 0.0 0.0)))))

(event `FinalRiddleAttach`
  (params (Component :type "SceneComponent Object Reference") (Actor :type "Actor Object Reference"))
  (`self.K2_AttachToComponent` Component "None" "SnapToTarget" "KeepWorld" "KeepWorld" false)
  (`PrimitiveComponent.SetSimulatePhysics` (`self.StaticMesh`) false)
  (set `self.AttachementOwner` Actor)
  (`KismetSystemLibrary.PrintString` "FinalRiddleAttach"))

(event `InputAction|Inspection`
  (params (Key :type "Key Structure"))
  (:`Pressed`
    (`KismetSystemLibrary.PrintString` "Hello")
    (bind _asbp_final_puzzle (cast `/Game/Blueprint/Puzzles/FinalPuzzle/BP_FinalPuzzle` (`self.OwnerPawn`)))
    (`self.Attach` (`/Game/Blueprint/Puzzles/FinalPuzzle/BP_FinalPuzzle.AttachmentPoint` _asbp_final_puzzle) _asbp_final_puzzle)
    (`self.Stop inspect` (0.0 0.0 0.0))))

(event `FinalRiddleDetach`
  (`self.K2_DetachFromActor` "KeepWorld" "KeepWorld" "KeepWorld")
  (set `self.AttachementOwner` null)
  (`KismetSystemLibrary.PrintString` "Final Riddle Detach Successful"))

(fn `UserConstructionScript`
  (`parent.UserConstructionScript`))