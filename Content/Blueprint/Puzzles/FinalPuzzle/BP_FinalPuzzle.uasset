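; Possessable final puzzle box that unlocks in two phases and is worked with the mouse cursor.
; Each Activate call enables that phase's actor collisions and opens lids with timeline-driven interpolation.
; While possessed, an attachment point tracks the deprojected cursor, and click traces grab items, attach them to interactables or drop them on the riddle tray.
; An Inspection input forwards to the held item, and M repossesses the player.
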(event `/Game/Blueprint/Puzzles/IBP_Interactions.Activate`
  (bind _meshtop (`self.MeshTop`))
  (bind _secondpuzzleupperlid (`self.SecondPuzzleUpperLid`))
  (bind _secondpuzzlelowerlid (`self.SecondPuzzleLowerLid`))
  (bind _secondpuzzlelowerlid_2 (`self.SecondPuzzleLowerLid`))
  (bind _secondarypuzzlelidrotspeed (`self.SecondaryPuzzleLidRotSpeed`))
  (bind _secondpuzzleupperlid_2 (`self.SecondPuzzleUpperLid`))
  ;[1 1 1] When key used, activate
  (switch `int` (`self.PuzzlePhase`)
    (:`0`
      (`|ExecutionSequence`
        (:`then_0`
          (bind (_direction _delta) (`Timeline|LidOpeningTimeline` :!via `PlayFromStart`)
            (:`Update`
              (bind _returnvalue (`self.CalcRotation` _delta _meshtop (`self.LidRotationSpeed`) (`self.MainLidOpenRot`)))
              (`SceneComponent.K2_SetWorldRotation` _meshtop _returnvalue false false))))
        (:`then_1`
          (`self.SetActorEnableCollision` true))
        (:`then_2`
          (for _array_element (`self.PuzzlePhase1Actors`)
            (`self.SetActorEnableCollision` _array_element true))
          (`/Engine/EditorBlueprintResources/StandardMacros.IncrementInt` (`self.PuzzlePhase`)))))
    (:`1`
      (`|ExecutionSequence`
        (:`then_0`
          (for _array_element_2 (`self.PuzzlePhase2Actors`)
            (`self.SetActorEnableCollision` _array_element_2 true)
            (`KismetSystemLibrary.PrintString` "Phase 2 Activated"))
          (`/Engine/EditorBlueprintResources/StandardMacros.IncrementInt` (`self.PuzzlePhase`)))
        (:`then_1`
          (bind (_direction_2 _delta_2) (`Timeline|SecondaryPuzzleLidRotation` :!via `PlayFromStart`)
            (:`Update`
              (`|ExecutionSequence`
                (:`then_0`
                  (bind _returnvalue_2 (`self.CalcRotation` _delta_2 _secondpuzzlelowerlid _secondarypuzzlelidrotspeed (`self.SecondaryLowerLidOpenRot`)))
                  (`SceneComponent.K2_SetWorldRotation` _secondpuzzlelowerlid _returnvalue_2 false false))
                (:`then_1`
                  (bind _returnvalue_3 (`self.CalcRotation` _delta_2 _secondpuzzleupperlid_2 _secondarypuzzlelidrotspeed (`self.SecondaryUpperLidOpenRot`)))
                  (`SceneComponent.K2_SetWorldRotation` _secondpuzzleupperlid_2 _returnvalue_3 false false))))
            (:`Finished`
              (bind (_direction_3 _delta_3) (`Timeline|SecondaryPuzzleLidSlide` :!via `PlayFromStart`)
                (:`Update`
                  (`|ExecutionSequence`
                    (:`then_0`
                      (bind _newpos (`self.MoveObject` _secondpuzzleupperlid (- (`SceneComponent.K2_GetComponentLocation` _secondpuzzleupperlid) (0.0 -0.0 0.05)) _delta_3 (`self.SecondaryPuzzleLidMovementSpeed`)))
                      (`SceneComponent.K2_SetWorldLocation` _secondpuzzleupperlid _newpos false false))
                    (:`then_1`
                      (bind _newpos_2 (`self.MoveObject` _secondpuzzlelowerlid_2 (- (`SceneComponent.K2_GetComponentLocation` _secondpuzzlelowerlid_2) (0.0 0.0 0.05)) _delta_3 (`self.SecondaryPuzzleLidMovementSpeed`)))
                      (`SceneComponent.K2_SetWorldLocation` _secondpuzzlelowerlid_2 _newpos_2 false false))))))))))))

(event `self.ReceiveBeginPlay`
  ;[1 1 1] Disabled puzzle phase collisions
  (`|ExecutionSequence`
    (:`then_0`
      (for _array_element (`self.PuzzlePhase1Actors`)
        (`self.SetActorEnableCollision` _array_element false)))
    (:`then_1`
      (for _array_element_2 (`self.PuzzlePhase2Actors`)
        (`self.SetActorEnableCollision` _array_element_2 false)))))

(event `/Game/Blueprint/Puzzles/PianoPuzzle/BPI_Enter.Enter`
  (params (Player :type "/Game/Blueprint/Player/FirstPersonCharacter Object Reference"))
  ;[1 1 1] Possess/Unpossess
  (set `self.Player` Player)
  (`Controller.Possess` (`GameplayStatics.GetPlayerController` 0) self)
  (set `self.IsActive` true)
  (`self.PuzzleActivationSettings` true))

(event `Key|LeftMouseButton`
  (params (Key :type "Key Structure"))
  (bind (_worldlocation _worlddirection) (`PlayerController.DeprojectMousePositionToWorld` (`GameplayStatics.GetPlayerController` 0)))
  (bind _returnvalue (!= (`self.AttachedObject`) null))
  ;[1 1 1] Input Linetrace
  (:`Pressed`
    (bind (_outhit _returnvalue_2) (`KismetSystemLibrary.LineTraceSingle` _worldlocation (+ _worldlocation (* _worlddirection 100)) "TraceTypeQuery1" false (`|MakeArray` (`self.AttachedObject`) :!type "Actor Object Reference") "ForDuration"))
    (if (and _returnvalue_2 (== (`self.AttachedObject`) null))
      (bind (_bblockinghit _binitialoverlap _time _distance _location _impactpoint _normal _impactnormal _physmat _hitactor) (`GameplayStatics.BreakHitResult` _outhit))
      (bind _asbp_item_parent (cast `/Game/Blueprint/BP_ItemParent` _hitactor)
        (:`then`
          (message `/Game/Blueprint/IBP_Grabable.Grab` _hitactor self (`self.AttachmentPoint`))
          (set `self.AttachedObject` _asbp_item_parent))
        (:`CastFailed`
          (`KismetSystemLibrary.PrintString` "Cast Failed")))
      (elif (and (`KismetSystemLibrary.DoesImplementInterface` _hitactor "/Game/Blueprint/Puzzles/IBP_Interactions.IBP_Interactions_C") _returnvalue)
        (message `/Game/Blueprint/Puzzles/IBP_Interactions.Attach` _hitactor (`self.AttachedObject`) null)
        (set `self.AttachedObject` null)
        (elif (and _returnvalue (== _hitactor (`self.RiddleTray`)))
          (message `/Game/Blueprint/IBP_Grabable.Drop` (`self.AttachedObject`))
          (`self.K2_SetActorLocation` (`self.AttachedObject`) _impactpoint false false)
          (set `self.AttachedObject` null))))))

(event `Key|M`
  (params (Key :type "Key Structure"))
  ;[1 1 1] Possess/Unpossess
  (:`Pressed`
    (`Controller.Possess` (`GameplayStatics.GetPlayerController` 0) (`self.Player`))
    (set `self.IsActive` false)
    (`self.PuzzleActivationSettings` false)))

(event `self.ReceiveTick`
  (params (DeltaSeconds :type "Float (single-precision)"))
  ;[1 1 1] Update Things & Stuff (Yeah I don't know exactly myself)
  (if (`self.IsActive`)
    (`self.UpdateAttachmentPointPos`)))

(event `InputAction|Inspection`
  (params (Key :type "Key Structure"))
  (bind _attachedobject (`self.AttachedObject`))
  ;[1 1 1] Activate Inspection
  (:`Pressed`
    (if (!= _attachedobject null)
      (message `/Game/Blueprint/IBP_Grabable.PawnInteractWith` _attachedobject self))))

(fn `PuzzleActivationSettings`
  (params (ShowCursor :type Boolean))
  (set `PlayerController.bShowMouseCursor` ShowCursor (`GameplayStatics.GetPlayerController` 0)))

(fn `UpdateAttachmentPointPos`
  (bind (_worldlocation _worlddirection _returnvalue) (`PlayerController.DeprojectMousePositionToWorld` (`GameplayStatics.GetPlayerController` 0)))
  (if _returnvalue
    (`SceneComponent.K2_SetWorldLocation` (`self.AttachmentPoint`) (+ _worldlocation (* _worlddirection 10)) false false)))

(fn `UserConstructionScript`
  (`self.SetActorEnableCollision` false))