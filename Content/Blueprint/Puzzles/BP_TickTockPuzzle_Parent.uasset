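; Parent Blueprint for a TickTock puzzle, apparently an unfinished mouse-drag rotation mechanic.
; OnMouseDown sets IsRotating and stores the cursor position, and OnMouseUp clears the flag.
; Tick is empty, and the disconnected rotation logic computes a mouse offset but only sets RotatingMiddleD to zero rotation.
; A delayed MultiGate that prints a debug count is also disconnected.
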(event `self.ReceiveTick`
  (params (DeltaSeconds :type "Float (single-precision)")))

(fn `OnMouseDown`
  (bind (_locationx _locationy) (`PlayerController.GetMousePosition` (`GameplayStatics.GetPlayerController` 0)))
  (set `self.isRotating` true)
  (set `self.MousePos` (`KismetMathLibrary.MakeVector2D` _locationx _locationy)))

(fn `OnMouseUp`
  (set `self.isRotating` false))

(fn `UserConstructionScript`)