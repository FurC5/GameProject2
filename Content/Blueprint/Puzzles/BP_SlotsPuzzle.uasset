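; BP_SlotsPuzzle is a puzzle manager that checks whether each slot in its Slots array holds the actor with the expected ID.
; On BeginPlay it registers itself as OwnerPuzzle on each slot.
; CheckPuzzle compares each slot's attached actor ID to that entry's ID, stopping at the first mismatch.
; When all match, it calls ActivateMessage on ActorToActivate.
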(event `self.ReceiveBeginPlay`
  (for _array_element (`self.Slots`)
    (set `/Game/Blueprint/Puzzles/BP_MemorySlot.OwnerPuzzle` self (break `/Game/Blueprint/Puzzles/Struct_SlotPuzzleMemory` _array_element))))

(event `CheckPuzzle`
  ;[1 1 1] CheckSlotsAreCorrect
  (for _array_element (`self.Slots`) :!label _label
    (bind (_slot _id) (break `/Game/Blueprint/Puzzles/Struct_SlotPuzzleMemory` _array_element))
    (if (`KismetStringLibrary.EqualEqual_StrStr` (`/Game/Blueprint/Puzzles/BP_PuzzleActor_Parent.ID` (`/Game/Blueprint/Puzzles/BP_MemorySlot.AttachedActor` _slot)) _id)
      (set `self.CorrectID` true)
      (else
        (set `self.CorrectID` false)
        (`self.BreakLoop`))))
  (if (`self.CorrectID`)
    (message `/Game/Blueprint/Puzzles/IBP_Interactions.Activate` (`self.ActorToActivate`))))

(event `BreakLoop`
  ;[1 1 1] CheckSlotsAreCorrect
  (goto _label :!via `Break`))

(fn `UserConstructionScript`)