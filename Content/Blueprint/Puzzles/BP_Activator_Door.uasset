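; Puzzle door actor that swings its mesh in yaw toward a stop rotation on Activate and back to its starting yaw on Deactivate.
; The MoveDoor timeline plays forward or in reverse, driving constant-rate rotation interpolation scaled by OpeningSpeed, with opening and closing sounds.
; Paired DoOnce gates block retriggering, resetting when the timeline finishes.
; Attach always returns false, and an unfinished yaw-difference calculation is left unconnected.
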(event `self.ReceiveBeginPlay`
  (bind (_returnvalue_roll _returnvalue_pitch _returnvalue_yaw) (`KismetMathLibrary.BreakRotator` (`SceneComponent.K2_GetComponentRotation` (`self.Mesh`))))
  (set `self.OriginalYaw` _returnvalue_yaw))

(event `/Game/Blueprint/Puzzles/IBP_Interactions.Deactivate`
  (bind (_doorstoprot_roll _doorstoprot_pitch _doorstoprot_yaw) (`KismetMathLibrary.BreakRotator` (`self.DoorStopRot`)))
  (bind _returnvalue (`SceneComponent.K2_GetComponentRotation` (`self.Mesh`)))
  ;[1 1 1] Rotate Door
  (`/Engine/EditorBlueprintResources/StandardMacros.DoOnce` false :!label _label
    (:`Completed`
      (`|ExecutionSequence`
        (:`then_0`
          (bind (_direction _movementfloat) (`Timeline|MoveDoor` :!via `ReverseFromEnd` :!label _label_2)
            (:`Update`
              (switch `ETimelineDirection` _direction
                (:`Forward`
                  (bind _returnvalue_2 (* _movementfloat (`self.OpeningSpeed`)))
                  (bind (_returnvalue_roll _returnvalue_pitch _returnvalue_yaw) (`KismetMathLibrary.BreakRotator` (`KismetMathLibrary.RInterpTo_Constant` (`SceneComponent.K2_GetComponentRotation` (`self.Mesh`)) (`self.DoorStopRot`) _movementfloat _returnvalue_2)))
                  (`SceneComponent.K2_SetWorldRotation` (`self.Mesh`) (`KismetMathLibrary.MakeRotator` 0.0 0.0 _returnvalue_yaw) false false))
                (:`Backward`
                  (bind (_returnvalue_roll_2 _returnvalue_pitch_2 _returnvalue_yaw_2) (`KismetMathLibrary.BreakRotator` (`KismetMathLibrary.RInterpTo_Constant` _returnvalue (`KismetMathLibrary.MakeRotator` (.roll _returnvalue) (.pitch _returnvalue) (`self.OriginalYaw`)) _movementfloat _returnvalue_2)))
                  (`SceneComponent.K2_SetWorldRotation` (`self.Mesh`) (`KismetMathLibrary.MakeRotator` 0.0 0.0 _returnvalue_yaw_2) false false))))
            (:`Finished`
              (`|ExecutionSequence`
                (:`then_0`
                  (goto _label :!via `Reset`))
                (:`then_1`
                  (goto _label_3 :!via `Reset`))))))
        (:`then_1`
          (`GameplayStatics.PlaySoundAtLocation` (`self.DoorClosingSound`) (`SceneComponent.K2_GetComponentLocation` (`self.Mesh`)) (struct) 1.0 1.0 0.0 "/Game/Audio/SoundFX/Environment/Outdoors/Rain/AT_RainArea.AT_RainArea" null null))))))

(event `/Game/Blueprint/Puzzles/IBP_Interactions.Activate`
  (bind (_doorstoprot_roll _doorstoprot_pitch _doorstoprot_yaw) (`KismetMathLibrary.BreakRotator` (`self.DoorStopRot`)))
  ;[1 1 1] Rotate Door
  (`/Engine/EditorBlueprintResources/StandardMacros.DoOnce` false :!label _label_3
    (:`Completed`
      (`|ExecutionSequence`
        (:`then_0`
          (goto _label_2 :!via `PlayFromStart`))
        (:`then_1`
          (`GameplayStatics.PlaySoundAtLocation` (`self.DoorOpeningSound`) (`SceneComponent.K2_GetComponentLocation` (`self.Mesh`)) (struct) 1.0 1.0 0.0 "/Game/Audio/SoundFX/Environment/Outdoors/Rain/AT_RainArea.AT_RainArea" null null))
        (:`then_2`
          (`KismetSystemLibrary.PrintString` (`KismetStringLibrary.Conv_DoubleToString` _doorstoprot_yaw)))))))

(fn `Attach`
  (params (Actor :type "/Game/Blueprint/BP_ItemParent Object Reference") (Inspection :type "/Game/Blueprint/Inspecting/BP_InspectionObject_1 Object Reference"))
  (returns (Attached :type Boolean))
  (return false))

(fn `UserConstructionScript`
  (`parent.UserConstructionScript`))