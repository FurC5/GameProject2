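; Puzzle door activator that swings its mesh toward a doorstop when activated.
; BeginPlay derives the target yaw from a negated look-at rotation between the mesh and DoorStop.
; Activate plays the MoveDoor timeline, adding a fraction of the absolute remaining yaw difference, scaled by the curve, each update until within tolerance.
; It prints each step for debugging; the saved original yaw is unused, so no closing logic exists.
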(event `self.ReceiveBeginPlay`
  (bind (_returnvalue_roll _returnvalue_pitch _returnvalue_yaw) (`KismetMathLibrary.BreakRotator` (`SceneComponent.K2_GetComponentRotation` (`self.Mesh`))))
  ;[1 1 1] BeginPlay/SetDoorstopPos
  (set `self.DoorStopRot` (`KismetMathLibrary.NegateRotator` (`KismetMathLibrary.FindLookAtRotation` (`SceneComponent.K2_GetComponentLocation` (`self.Mesh`)) (`SceneComponent.K2_GetComponentLocation` (`self.DoorStop`)))))
  (set `self.OriginalYaw` _returnvalue_yaw))

(event `/Game/Blueprint/Puzzles/IBP_Interactions.Activate`
  (bind (_doorstoprot_roll _doorstoprot_pitch _doorstoprot_yaw) (`KismetMathLibrary.BreakRotator` (`self.DoorStopRot`)))
  (bind (_returnvalue_roll _returnvalue_pitch _returnvalue_yaw) (`KismetMathLibrary.BreakRotator` (`SceneComponent.K2_GetComponentRotation` (`self.Mesh`))))
  (`|ExecutionSequence`
    (:`then_0`
      ;[1 1 1] Rotate Door
      (bind (_direction _movementfloat) (`Timeline|MoveDoor` :!via `PlayFromStart`)
        (:`Update`
          (if (not (`KismetMathLibrary.NearlyEqual_FloatFloat` _returnvalue_yaw _doorstoprot_yaw 0.5))
            (bind _returnvalue (* (/ (`KismetMathLibrary.Abs` (- _returnvalue_yaw _doorstoprot_yaw)) 100.0) _movementfloat))
            (`KismetSystemLibrary.PrintString` (`KismetTextLibrary.Conv_TextToString` (`|FormatText` "Timeline Value {V}" _returnvalue)))
            (`SceneComponent.K2_SetWorldRotation` (`self.Mesh`) (`KismetMathLibrary.MakeRotator` 0.0 0.0 (+ _returnvalue_yaw _returnvalue)) false false)))))))

(fn `UserConstructionScript`
  (`parent.UserConstructionScript`))