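; BP_SlotsPuzzle is a puzzle that activates a target actor when every slot holds the item with the expected ID.
; On BeginPlay it registers itself as the owner of each slot in its Slots array.
; CheckPuzzle compares each slot's attached actor ID with that entry's ID, breaking on the first empty or wrong slot.
; If all match, it sends ActivateMessage to ActorToActivate.
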(event `self.ReceiveBeginPlay`
  (for _array_element (`self.Slots`)
    (set `/Game/Blueprint/Puzzles/SequencePuzzle/BP_MemorySlot.OwnerPuzzle` self (break `/Game/Blueprint/Puzzles/SequencePuzzle/Struct_SlotPuzzleMemory` _array_element))))

(event `CheckPuzzle`
  ;[1 1 1] CheckSlotsAreCorrect
  (for _array_element (`self.Slots`) :!label _label
    (bind (_slot _id) (break `/Game/Blueprint/Puzzles/SequencePuzzle/Struct_SlotPuzzleMemory` _array_element))
    (bind _attachedactor (`/Game/Blueprint/Puzzles/SequencePuzzle/BP_MemorySlot.AttachedActor` _slot))
    (if (!= _attachedactor null)
      (if (`KismetStringLibrary.EqualEqual_StrStr` (`/Game/Blueprint/BP_ItemParent.ID` _attachedactor) _id)
        (set `self.CorrectID` true)
        (else
          (set `self.CorrectID` false :!label _label_2)
          (`self.BreakLoop`)))
      (else
        (goto _label_2))))
  (if (`self.CorrectID`)
    (message `/Game/Blueprint/Puzzles/IBP_Interactions.Activate` (`self.ActorToActivate`))))

(event `BreakLoop`
  ;[1 1 1] CheckSlotsAreCorrect
  (goto _label :!via `Break`))

(fn `UserConstructionScript`)