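; Memory slot for a sequence puzzle that holds one attached actor and reports to its owning puzzle.
; Attach accepts an actor only if it carries both the puzzle's and the slot's attachment tags, gated by an AttachedActor check.
; It stores the actor, triggers CheckPuzzle, prints debug text, then sends drop and grab messages to move it onto AttachPoint.
; Detach only clears the stored reference.
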(event `/Game/Blueprint/Puzzles/IBP_Interactions.Detach`
  (set `self.AttachedActor` null))

(event `/Game/Blueprint/Puzzles/IBP_Interactions.Attach`
  (params (Actor :type "/Game/Blueprint/BP_ItemParent Object Reference"))
  (bind _tags (`Actor.Tags` Actor))
  (bind _attachedactor (`self.AttachedActor`))
  ;[1 1 1] Attach Actor To Memory Slot
  (if (and (`KismetArrayLibrary.Array_Contains` _tags (`/Game/Blueprint/Puzzles/SequencePuzzle/BP_SlotsPuzzle.AttachementTag` (`self.OwnerPuzzle`))) (`KismetArrayLibrary.Array_Contains` _tags (`self.AttachementTag`)) (== (`self.AttachedActor`) null))
    (set `self.AttachedActor` Actor)
    (`/Game/Blueprint/Puzzles/SequencePuzzle/BP_SlotsPuzzle.CheckPuzzle` (`self.OwnerPuzzle`))
    (`KismetSystemLibrary.PrintString` (`KismetTextLibrary.Conv_TextToString` (`|FormatText` "{Me} is holding {Obj}" (`KismetSystemLibrary.GetDisplayName` self) (`KismetSystemLibrary.GetDisplayName` (`self.AttachedActor`)))))
    (message `/Game/Blueprint/IBP_Grabable.Drop` _attachedactor)
    (message `/Game/Blueprint/IBP_Grabable.Grab` _attachedactor self (`self.AttachPoint`))))

(fn `UserConstructionScript`)